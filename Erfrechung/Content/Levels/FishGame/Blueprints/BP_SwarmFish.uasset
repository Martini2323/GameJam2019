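; Fish actor for the fish level that swims in a boids-style swarm and flees the BP_FishLevelPawn.
; Each tick it sums forward, flee, world-origin pull and flock vectors, sets the root's physics velocity and turns to face it.
; Flock scans every BP_SwarmFish per tick, using avoidance and recognition radii for separation, cohesion and alignment.
; Alignment is weighted by neighbor count rather than a tunable factor.
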(event EventTick
  (params (DeltaSeconds :type Float%20%28single-precision%29))
  (bind _returnvalue (Transformation|GetActorLocation))
  (Variables|Default|SetForce (* (+ (CallFunction|GoForward) (CallFunction|Flee) (CallFunction|GoMid) (CallFunction|Flock)) (/ (Variables|Default|GetSpeedMultiplier) 4.0)))
  (Physics|SetPhysicsLinearVelocity (Variables|Default|GetRoot) (Variables|Default|GetForce) false "None")
  (Transformation|SetActorRotation (Math|Interpolation|RInterpTo (Transformation|GetActorRotation) (Math|Rotator|FindLookatRotation _returnvalue (+ _returnvalue (Variables|Default|GetForce))) DeltaSeconds 5e+01)))

(fn ConstructionScript)

(fn GoMid
  (return (* (Math|Vector|Normalize (- (Math|Vector|MakeVector 0.0 0.0 0.0) (Transformation|GetActorLocation))) (Variables|Default|GetMid))))

(fn Flee
  (bind _returnvalue (Actor|GetActorOfClass "/Game/Levels/FishGame/Blueprints/BP_FishLevelPawn.BP_FishLevelPawn_C"))
  (return (* (Math|Vector|Normalize (- (Transformation|GetActorLocation) (Transformation|GetActorLocation _returnvalue))) (Variables|Default|GetFleeFactor))))

(fn GoForward
  (return (* (Transformation|GetActorForwardVector) (Variables|Default|GetForward))))

(fn Flock
  (bind _returnvalue (Transformation|GetActorLocation))
  (bind _outactors (Actor|GetAllActorsOfClass "BP_SwarmFish_C"))
  (for _array_element _outactors
    (if (Math|Float|InRange(Float) (Math|Vector|Distance(Vector) (Transformation|GetActorLocation _array_element) _returnvalue) 0.0 (Variables|Default|GetAvoidance) false)
      (LocalVariables|SetAvoidanceCtn (+ (LocalVariables|GetAvoidanceCtn) 1))
      (LocalVariables|SetAvoidanceDir (- (LocalVariables|GetAvoidanceDir) (- (Transformation|GetActorLocation _array_element) _returnvalue)))
      (LocalVariables|SetAverageDir (+ (LocalVariables|GetAverageDir) (Transformation|GetActorForwardVector _array_element)) :!label _label)
      (elif (Math|Float|InRange(Float) (Math|Vector|Distance(Vector) (Transformation|GetActorLocation _array_element) _returnvalue) (Variables|Default|GetAvoidance) (Variables|Default|GetRecognition) false)
        (LocalVariables|SetCtn (+ (LocalVariables|GetCtn) 1))
        (LocalVariables|SetAveragePos (+ (LocalVariables|GetAveragePos) (Transformation|GetActorLocation _array_element)))
        (goto _label))))
  (if (> (LocalVariables|GetCtn) 0)
    (LocalVariables|SetFlockForce (* (Math|Vector|Normalize (- (/ (LocalVariables|GetAveragePos) (LocalVariables|GetCtn)) (Transformation|GetActorLocation))) (Variables|Default|GetCohesion))))
  (if (> (LocalVariables|GetAvoidanceCtn) 0)
    (LocalVariables|SetFlockForce (+ (LocalVariables|GetFlockForce) (* (Math|Vector|Normalize (LocalVariables|GetAvoidanceDir)) (Variables|Default|GetSeperation)))))
  (if (> (+ (LocalVariables|GetCtn) (LocalVariables|GetAvoidanceCtn)) 0)
    (LocalVariables|SetFlockForce (+ (LocalVariables|GetFlockForce) (* (Math|Vector|Normalize (LocalVariables|GetAverageDir)) (+ (LocalVariables|GetCtn) (LocalVariables|GetAvoidanceCtn))))))
  (return (/ (LocalVariables|GetFlockForce) 3)))