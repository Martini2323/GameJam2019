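; Player pawn for the fish minigame level, scaled down on construction and steered by the mouse.
; Each tick it projects the cursor onto the Z=0 plane and uses that point's absolute XY as the Sphere's physics velocity.
; Rotation interpolates quickly toward that direction of travel.
; Tick also polls for BP_SwarmFish actors and, when none remain, calls CallFishGameWon instead of updating movement.
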(event EventBeginPlay)

(event Collision|EventActorBeginOverlap
  (params (OtherActor :type Actor%20Object%20Reference)))

(event EventTick
  (params (DeltaSeconds :type Float%20%28single-precision%29))
  (bind _returnvalue (Game|GetPlayerController 0))
  (bind _returnvalue_2 (Transformation|GetActorLocation))
  (bind (_worldlocation _worlddirection) (Game|Player|ConvertMouseLocationToWorldSpace _returnvalue))
  (bind _z (Math|Vector|BreakVector _worldlocation))
  (bind _z_2 (Math|Vector|BreakVector _worlddirection))
  (bind _returnvalue_3 (/ _z _z_2))
  (bind _returnvalue_4 (* _worlddirection _returnvalue_3))
  (bind _returnvalue_5 (Math|Vector|NegateVector _returnvalue_4))
  (bind _returnvalue_6 (+ _worldlocation _returnvalue_5))
  (bind _returnvalue_7 (Math|Vector|MakeVector (.x _returnvalue_6) (.y _returnvalue_6) 0.0))
  (bind _outactors (Actor|GetAllActorsOfClass "/Game/Levels/FishGame/Blueprints/BP_SwarmFish.BP_SwarmFish_C"))
  (if (== (Utilities|Array|Length _outactors) 0)
    (Default|CallFishGameWon)
    (else
      (Class|PrimitiveComponent|SetAllPhysicsLinearVelocity (Variables|Default|GetSphere) _returnvalue_7 false)
      (Transformation|SetActorRotation (Math|Interpolation|RInterpTo (Transformation|GetActorRotation) (Math|Rotator|FindLookatRotation _returnvalue_2 (+ (* _returnvalue_7 DeltaSeconds) _returnvalue_2)) DeltaSeconds 5e+01)))))

(fn ConstructionScript
  (Transformation|SetActorScale3D "0.400000,0.400000,0.400000"))