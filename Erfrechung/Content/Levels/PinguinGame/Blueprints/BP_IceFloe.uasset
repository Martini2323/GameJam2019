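; BP_IceFloe is an ice floe in the penguin minigame that carries a penguin and melts under a blower.
; On BeginPlay it picks a random mesh and yaw, then either spawns a penguin on itself and randomizes its scale or destroys itself by spawn probability.
; Overlap with BP_Blower shrinks it on Tick; below a size threshold the penguin gets physics, and the floe hides, splashes with sound and destroys itself.
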(event OnComponentBeginOverlap(Floe)
  (params (OverlappedComponent :type Primitive%20Component%20Object%20Reference) (OtherActor :type Actor%20Object%20Reference) (OtherComp :type Primitive%20Component%20Object%20Reference) (OtherBodyIndex :type Integer) (bFromSweep :type Boolean) (SweepResult :type Hit%20Result%20Structure%20%28by%20ref%29))
  (Utilities|Casting|CastToBP_Blower OtherActor)
  (Variables|Default|SetShrinking true))

(event OnComponentEndOverlap(Floe)
  (params (OverlappedComponent :type Primitive%20Component%20Object%20Reference) (OtherActor :type Actor%20Object%20Reference) (OtherComp :type Primitive%20Component%20Object%20Reference) (OtherBodyIndex :type Integer))
  (Utilities|Casting|CastToBP_Blower OtherActor)
  (Variables|Default|SetShrinking false))

(event EventBeginPlay
  (bind _returnvalue (Math|Random|RandomRotator false))
  (bind _floes (Variables|Default|GetFloes))
  (bind _returnvalue_2 (Math|Rotator|MakeRotator 0.0 0.0 (.yaw _returnvalue)))
  (Components|StaticMesh|SetStaticMesh (Variables|Default|GetFloe) (Utilities|Array|Get(acopy) _floes (Math|Random|RandomIntegerinRange 0 (- (Utilities|Array|Length _floes) 1))))
  (Transformation|SetWorldRotation (Variables|Default|GetFloe) _returnvalue_2 false false)
  (if (CallFunction|ShouldSpawn)
    (bind _returnvalue_3 (Game|SpawnActorfromClass "/Game/Levels/PinguinGame/Blueprints/BP_Pinguin.BP_Pinguin_C" (Math|Transform|MakeTransform (Transformation|GetWorldLocation (Variables|Default|GetFloe self)) _returnvalue_2 "1,1,1") "Undefined" 0 0))
    (Variables|Default|SetPinguin _returnvalue_3)
    (Transformation|SetWorldScale3D (Variables|Default|GetFloe) (Math|Conversions|ToVector(Float) (Math|Random|RandomFloatinRange 0.4 0.6)))
    (else
      (Actor|DestroyActor))))

(event EventTick
  (params (DeltaSeconds :type Float%20%28single-precision%29))
  (bind _meltspeed (Variables|Default|GetMeltSpeed))
  (bind _floe (Variables|Default|GetFloe))
  (bind _floe_2 (Variables|Default|GetFloe))
  (bind _returnvalue (Transformation|GetWorldTransform _floe_2))
  (bind _returnvalue_2 (Transformation|GetWorldScale _floe))
  (bind _returnvalue_3 (* DeltaSeconds _meltspeed))
  (bind _returnvalue_4 (- (.x _returnvalue_2) _returnvalue_3))
  (if (and (not (Variables|Default|GetDone)) (Variables|Default|GetShrinking))
    (Transformation|SetWorldScale3D (Variables|Default|GetFloe) (Math|Vector|MakeVector _returnvalue_4 _returnvalue_4 _returnvalue_4))
    (if (< (.x _returnvalue_2) 0.1)
      (Variables|Default|SetDone true)
      (Physics|SetSimulatePhysics (Variables|/Game/Levels/PinguinGame/Blueprints/BP_Pinguin.BP_Pinguin_C|GetPinguin (Variables|Default|GetPinguin)) true) ; World Kill Z Handles Destroy
      (Rendering|SetVisibility (Variables|Default|GetFloe) false false)
      (Effects|SpawnEmitteratLocation "/Game/Levels/PinguinGame/P_Splash.P_Splash" (.location _returnvalue) (.rotation _returnvalue) (* (.scale _returnvalue) 2e+01) false)
      (Utilities|FlowControl|Delay 0.2)
      (AddComponent|AddAudioComponent false)
      (Utilities|FlowControl|Delay 1.0)
      (Actor|DestroyActor))))

(fn ConstructionScript)

(fn ShouldSpawn
  (return (< (Math|Random|RandomFloat) (Variables|Default|GetSpawnProbability))))