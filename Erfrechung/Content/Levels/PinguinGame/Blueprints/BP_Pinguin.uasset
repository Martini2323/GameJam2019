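; BP_Pinguin is a penguin actor for the PinguinGame level that gets a random look and a wiggling motion.
; On BeginPlay, one random index picks the body mesh and the matching mesh shared by both wings.
; After a random delay, which offsets the start of each instance, the Wiggle timeline plays and adds its value to the body's current world pitch on every update.
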(event EventBeginPlay
  (bind _pinguin (Variables|Default|GetPinguin))
  (bind _returnvalue (Transformation|GetWorldRotation _pinguin))
  (Variables|Default|SetIndex (Math|Random|RandomIntegerinRange 0 (- (Utilities|Array|Length (Variables|Default|GetPinguins)) 1)))
  (Components|StaticMesh|SetStaticMesh (Variables|Default|GetPinguin) (Utilities|Array|Get(acopy) (Variables|Default|GetPinguins) (Variables|Default|GetIndex)))
  (Components|StaticMesh|SetStaticMesh (Variables|Default|GetLeftWing) (Utilities|Array|Get(acopy) (Variables|Default|GetWings) (Variables|Default|GetIndex)))
  (Components|StaticMesh|SetStaticMesh (Variables|Default|GetRightWing) (Utilities|Array|Get(acopy) (Variables|Default|GetWings) (Variables|Default|GetIndex)))
  (Utilities|FlowControl|Delay (Math|Random|RandomFloat))
  (bind _wiggle (Timeline|Wiggle Play)
    (:Update
      (Transformation|SetWorldRotation _pinguin (Math|Rotator|MakeRotator (.roll _returnvalue) (+ (.pitch _returnvalue) _wiggle) (.yaw _returnvalue)) false false))))

(fn ConstructionScript)