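; BP_Blower is a blower in the penguin minigame that follows the mouse cursor.
; Each Tick deprojects the cursor from player controller 0 and intersects that ray with the world Z=0 plane.
; The Blower component is moved to that point with a slight height offset, without sweep.
; The graph holds only this cursor tracking, with no blowing or force logic.
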(event EventTick
  (params (DeltaSeconds :type Float%20%28single-precision%29))
  (bind _returnvalue (Game|GetPlayerController 0))
  (bind (_worldlocation _worlddirection) (Game|Player|ConvertMouseLocationToWorldSpace _returnvalue))
  (bind _z (Math|Vector|BreakVector _worlddirection))
  (bind _z_2 (Math|Vector|BreakVector _worldlocation))
  (bind _returnvalue_2 (/ _z_2 _z))
  (bind _returnvalue_3 (* _worlddirection _returnvalue_2))
  (bind _returnvalue_4 (* _returnvalue_3 -1.0))
  (bind _returnvalue_5 (+ _worldlocation _returnvalue_4))
  (bind (_x _y _z_3) (Math|Vector|BreakVector _returnvalue_5))
  (Transformation|SetWorldLocation (Variables|Default|GetBlower) (Math|Vector|MakeVector _x _y (+ _z_3 2e+01)) false false))

(fn ConstructionScript)