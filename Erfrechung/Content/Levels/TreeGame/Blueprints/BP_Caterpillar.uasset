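; BP_Caterpillar is a steerable, constantly advancing caterpillar in the TreeGame level.
; While any BP_Tree actor exists, Tick overwrites the Cube's physics velocity along the actor's forward vector and applies frame-rate-scaled yaw from Torque.
; Left and right input actions set Torque to plus or minus RotationFactor, and releasing either resets it to zero.
; Any hit on the Cube turns the actor around to face the opposite direction.
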(event OnComponentHit(Cube)
  (params (HitComponent :type Primitive%20Component%20Object%20Reference) (OtherActor :type Actor%20Object%20Reference) (OtherComp :type Primitive%20Component%20Object%20Reference) (NormalImpulse :type Vector :default "0, 0, 0") (Hit :type Hit%20Result%20Structure%20%28by%20ref%29))
  (bind _returnvalue (Transformation|GetActorLocation))
  (Transformation|SetActorRotation (Math|Rotator|FindLookatRotation _returnvalue (+ _returnvalue (Math|Vector|NegateVector (Transformation|GetActorForwardVector))))))

(event EventBeginPlay)

(event Collision|EventActorBeginOverlap
  (params (OtherActor :type Actor%20Object%20Reference)))

(event EventTick
  (params (DeltaSeconds :type Float%20%28single-precision%29))
  (bind _outactors (Actor|GetAllActorsOfClass "/Game/Levels/TreeGame/Blueprints/BP_Tree.BP_Tree_C"))
  (if (not (== (Utilities|Array|Length _outactors) 0))
    (Physics|SetPhysicsLinearVelocity (Variables|Default|GetCube) (* (Transformation|GetActorForwardVector) (Variables|Default|GetSpeed)) false "None")
    (Class|Actor|AddActorWorldRotation (Math|Rotator|MakeRotator 0.0 0.0 (* (Variables|Default|GetTorque) DeltaSeconds)))))

(event Input|ActionEvents|InputActionInput_KeyLeft
  (params (Key :type Key%20Structure :default "None"))
  (:Pressed
    (Variables|Default|SetTorque (* (Variables|Default|GetRotationFactor) -1.0)))
  (:Released
    (Variables|Default|SetTorque 0.0)))

(event Input|ActionEvents|InputActionInput_KeyRight
  (params (Key :type Key%20Structure :default "None"))
  (:Pressed
    (Variables|Default|SetTorque (Variables|Default|GetRotationFactor)))
  (:Released
    (Variables|Default|SetTorque 0.0)))

(fn ConstructionScript)