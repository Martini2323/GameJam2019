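; Blueprint for a button-mashing oil pumping minigame, where repeated presses of an input action drive an animated skeletal mesh until the game is won.
; On BeginPlay it derives the required press count from the game instance's difficulty and freezes the animation.
; Each press speeds up the animation proportionally toward a maximum, and the first press starts a pump-jack sound.
; Reaching the target stops the sound and calls the oil game win.
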(event EventBeginPlay
  (bind _asbp_erfrecht_game_instance (Utilities|Casting|CastToBP_ErfrechtGameInstance (Game|GetGameInstance)))
  (Variables|Default|SetPressesNeeded (* (Variables|/Game/BP_ErfrechtGameInstance.BP_ErfrechtGameInstance_C|GetDifficulty _asbp_erfrecht_game_instance) 20))
  (Variables|/Script/Engine.SkeletalMeshComponent|SetGlobalAnimRateScale (Variables|Default|GetSkeletalMesh) 0.0)
  (Variables|Default|SetStep (/ (Variables|Default|GetMaxSpeed) (Math|Conversions|ToFloat(Integer) (Variables|Default|GetPressesNeeded)))))

(event Input|ActionEvents|InputActionInput_Action
  (params (Key :type Key%20Structure :default "None"))
  (:Pressed
    (if (== (Variables|Default|GetPressed) 0)
      (bind _returnvalue (Audio|SpawnSound2D "/Game/Levels/PumpingGame/pumpingJack_Cue.pumpingJack_Cue" 1.0 1.0 0.0 0))
      (Variables|Default|SetPumpingSound _returnvalue))
    (Variables|Default|SetPressed (+ (Variables|Default|GetPressed) 1))
    (Variables|/Script/Engine.SkeletalMeshComponent|SetGlobalAnimRateScale (Variables|Default|GetSkeletalMesh) (* (Variables|Default|GetPressed) (Variables|Default|GetStep)))
    (if (>= (Variables|Default|GetPressed) (Variables|Default|GetPressesNeeded))
      (Utilities|IsValid (Variables|Default|GetPumpingSound)
        (:Is%20Valid
          (Audio|Components|Audio|Stop (Variables|Default|GetPumpingSound)))
        (:Is%20Not%20Valid
          _))
      (Default|CallOilGameWon))))

(fn ConstructionScript)