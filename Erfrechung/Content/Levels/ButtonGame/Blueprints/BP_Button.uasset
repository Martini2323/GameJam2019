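; BP_Button is a one-shot pressable button actor for the ButtonGame level.
; Its Press function uses a Pressed flag to run only once, lowering the Button component, playing an explosion sound at the actor and removing the HUD widget if valid.
; The event graph is empty, so nothing in this Blueprint calls Press or sets the HUD reference.
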(event EventBeginPlay)

(event Collision|EventActorBeginOverlap
  (params (OtherActor :type Actor%20Object%20Reference)))

(fn ConstructionScript)

(fn Press
  (bind _button (Variables|Default|GetButton))
  (bind _hud (Variables|Default|GetHUD))
  (bind _relativelocation (Variables|/Script/Engine.SceneComponent|GetRelativeLocation _button))
  (if (not (Variables|Default|GetPressed))
    (Variables|Default|SetPressed true)
    (Transformation|SetRelativeLocation _button (Math|Vector|MakeVector (.x _relativelocation) (.y _relativelocation) (- (.z _relativelocation) 2e+01)) false false)
    (Audio|PlaySoundatLocation "/Game/StarterContent/Audio/Explosion01.Explosion01" (Transformation|GetActorLocation) "0, 0, 0" 1.0 1.0 0.0 0 0 0)
    (Utilities|IsValid _hud
      (:Is%20Valid
        (Widget|RemovefromParent _hud)))))